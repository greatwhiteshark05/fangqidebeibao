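; MyMyPawn is a pawn whose box trigger shows a UI widget on overlap.
; Begin overlap creates widget 123 and adds it to the player screen; end overlap fetches top-level instances of that class and calls RemoveExtensions on them, with debug prints on both.
; An unconnected graph, which never runs, would use Up, Down and F to highlight one of two buttons and print "turn on light" or "open door".
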(event `self.Box.OnComponentBeginOverlap`
  (params (OverlappedComponent :type "PrimitiveComponent Object Reference") (OtherActor :type "Actor Object Reference") (OtherComp :type "PrimitiveComponent Object Reference") (OtherBodyIndex :type Integer) (bFromSweep :type Boolean) (SweepResult :type "HitResult Structure (by ref)"))
  (`KismetSystemLibrary.PrintString` "Hello")
  (bind _returnvalue (`|CreateWidget` "/Game/blueprints/123.123_C"))
  (`UserWidget.AddToPlayerScreen` _returnvalue 0))

(event `self.Box.OnComponentEndOverlap`
  (params (OverlappedComponent :type "PrimitiveComponent Object Reference") (OtherActor :type "Actor Object Reference") (OtherComp :type "PrimitiveComponent Object Reference") (OtherBodyIndex :type Integer))
  (`KismetSystemLibrary.PrintString` "出来")
  (bind _foundwidgets (`WidgetBlueprintLibrary.GetAllWidgetsOfClass` "/Game/blueprints/123.123_C"))
  (`UserWidget.RemoveExtensions` _foundwidgets null))

(fn `UserConstructionScript`)